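; BP_MyPawn is a player pawn moved by applying torque to its static mesh, as in a rolling-ball controller.
; Forward/backward input feeds MoveFB for Y-axis torque, while left/right input applies negated X-axis torque directly.
; Both scale the axis value by Acceleration and apply it as an acceleration change, ignoring mass.
; An Evaluate acceleration graph branches on a boolean and checks Acceleration is non-negative, but neither input event uses it.
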(event Input|AxisEvents|InputAxisMoveForwards/Backwards
  (params (AxisValue :type Float%20%28single-precision%29))
  (CallFunction|MoveF/B AxisValue))

(event Input|AxisEvents|InputAxisMoveLeft/Right
  (params (AxisValue :type Float%20%28single-precision%29))
  (Class|PrimitiveComponent|AddTorqueinRadians (Variables|Default|GetStaticMesh) (Math|Vector|MakeVector (* (* AxisValue (Variables|Default|GetAcceleration)) -1.0) 0.0 0.0) "None" true))

(fn ConstructionScript)

(fn MoveF/B
  (params (A :type Float%20%28single-precision%29))
  (Class|PrimitiveComponent|AddTorqueinRadians (Variables|Default|GetStaticMesh) (Math|Vector|MakeVector 0.0 (* A (Variables|Default|GetAcceleration)) 0.0) "None" true))