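; BP_Collectible is a pickup actor that animates into the player when the player pawn overlaps it.
; On overlap it stores its scale and location, then plays a timeline that lerps scale toward DestinationScale and position toward the player.
; The move target is re-read each update, so the pickup homes in on a moving player.
; When the timeline finishes, it calls PlayerCollected and destroys itself.
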(event Collision|EventActorBeginOverlap
  (params (OtherActor :type Actor%20Object%20Reference))
  (if (== OtherActor (Game|Player|GetPlayerPawn 0))
    (CallFunction|SetStartingValues)
    (bind (_direction _scale_progress _movement_progress) (Timeline|Collection%20Timeline Play)
      (:Update
        (CallFunction|ScaleCollectible _scale_progress)
        (CallFunction|MovetoPlayer _movement_progress))
      (:Finished
        (Default|CallPlayerCollected)
        (Actor|DestroyActor)))))

(fn ConstructionScript)

(fn ScaleCollectible
  (params (Alpha :type Float%20%28single-precision%29))
  (Transformation|SetActorScale3D (Math|Vector|Lerp(Vector) (Variables|Default|GetStartScale) (Variables|Default|GetDestination%20Scale) Alpha)))

(fn SetStartingValues
  (Variables|Default|SetStartScale (Transformation|GetActorScale3D))
  (Variables|Default|SetStart%20Location (Transformation|GetActorLocation)))

(fn MovetoPlayer
  (params (Alpha :type Float%20%28single-precision%29))
  (Transformation|SetActorLocation (Math|Vector|Lerp(Vector) (Variables|Default|GetStart%20Location) (Transformation|GetActorLocation (Game|Player|GetPlayerPawn 0)) Alpha) false false))